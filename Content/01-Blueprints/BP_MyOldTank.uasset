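; BP_MyOldTank is a player-controlled tank with basic drive and turn movement via Enhanced Input.
; On BeginPlay it adds the IMC_Tank mapping context to the first player controller's input subsystem.
; IA_PlayerMovement moves the actor along its local forward axis with a collision sweep and yaws it, scaled by Speed, TurnRate and delta time.
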(event Input|EnhancedActionEvents|EnhancedInputActionIA_PlayerMovement
  (params (ActionValue :type Vector%202D%20Structure) (ElapsedSeconds :type Float%20%28double-precision%29) (TriggeredSeconds :type Float%20%28double-precision%29) (InputAction :type Input%20Action%20Object%20Reference :default "/Game/01-Blueprints/Inputs/TankActions/IA_PlayerMovement.IA_PlayerMovement"))
  (bind _returnvalue (Utilities|Time|GetWorldDeltaSeconds))
  (Variables|Default|SetDeltaLocation (Math|Vector|MakeVector (* (.y ActionValue) (Variables|Default|GetSpeed) _returnvalue) 0.0 0.0))
  (Transformation|AddActorLocalOffset (Variables|Default|GetDeltaLocation) true false)
  (Variables|Default|SetDeltaRotation (Math|Rotator|MakeRotator 0.0 0.0 (* (.x ActionValue) (Variables|Default|GetTurnRate) _returnvalue)))
  (Transformation|AddActorLocalRotation (Variables|Default|GetDeltaRotation) false false))

(event EventBeginPlay
  (bind _returnvalue (Game|GetPlayerController 0))
  (bind _returnvalue_2 (PlayerController|LocalPlayerSubsystems|GetEnhancedInputLocalPlayerSubsystem _returnvalue))
  (Utilities|IsValid _returnvalue
    (:Is%20Valid
      (Utilities|IsValid _returnvalue_2
        (:Is%20Valid
          (Input|AddMappingContext _returnvalue_2 "/Game/01-Blueprints/Inputs/IMC_Tank.IMC_Tank" 0 "(bIgnoreAllPressedKeysUntilRelease=True,bForceImmediately=False,bNotifyUserSettings=False)"))))))

(fn ConstructionScript)